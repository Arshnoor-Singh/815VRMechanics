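; VR bow actor that spawns BP_Arrow projectiles from its Arrow component, aligned to that component's forward vector.
; A looping timer started on BeginPlay fires arrows continuously, whether held or not, and IA_Shoot_Right also triggers a shot.
; GrabComponentSnap's grab and drop events toggle player input and add or remove a left- or right-hand Enhanced Input mapping context based on the holding hand.
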(event OnGrabbed(GrabComponentSnap)
  (Input|EnableInput (Game|GetPlayerController 0))
  (Input|AddMappingContext (PlayerController|LocalPlayerSubsystems|GetEnhancedInputLocalPlayerSubsystem (Game|GetPlayerController 0)) (select (Utilities|Enum|Equal(Enum) (Default|GetHeldbyHand (Variables|Default|GetGrabComponentSnap)) "Left") "/Game/VRTemplate/Input/IMC_BowLeft.IMC_BowLeft" "/Game/VRTemplate/Input/IMC_BowRight.IMC_BowRight") 1 "(bIgnoreAllPressedKeysUntilRelease=True,bForceImmediately=False)"))

(event OnDropped(GrabComponentSnap)
  (Input|DisableInput (Game|GetPlayerController 0))
  (Input|RemoveMappingContext (PlayerController|LocalPlayerSubsystems|GetEnhancedInputLocalPlayerSubsystem (Game|GetPlayerController 0)) (select (Utilities|Enum|Equal(Enum) (Default|GetHeldbyHand (Variables|Default|GetGrabComponentSnap)) "Left") "/Game/VRTemplate/Input/IMC_BowLeft.IMC_BowLeft" "/Game/VRTemplate/Input/IMC_BowRight.IMC_BowRight") "(bIgnoreAllPressedKeysUntilRelease=True,bForceImmediately=False)"))

(event Custom|Fire
  (bind _arrow (Variables|Default|GetArrow))
  (Game|SpawnActorfromClass "/Game/VRTemplate/Blueprints/BP_Arrow.BP_Arrow_C" (Math|Transform|MakeTransform (Transformation|GetWorldLocation _arrow) (Math|Conversions|RotationFromXVector (Math|Vector|GetForwardVector _arrow))) "Undefined" "MultiplyWithRoot" 0 0))

(event Input|EnhancedActionEvents|EnhancedInputActionIA_Shoot_Right
  (params (ActionValue :type Boolean) (ElapsedSeconds :type Float%20%28double-precision%29) (TriggeredSeconds :type Float%20%28double-precision%29) (InputAction :type Input%20Action%20Object%20Reference :default "/Game/VRTemplate/Input/Actions/IA_Shoot_Right.IA_Shoot_Right"))
  (bind _arrow (Variables|Default|GetArrow))
  (:Started
    (Game|SpawnActorfromClass "/Game/VRTemplate/Blueprints/BP_Arrow.BP_Arrow_C" (Math|Transform|MakeTransform (Transformation|GetWorldLocation _arrow) (Math|Conversions|RotationFromXVector (Math|Vector|GetForwardVector _arrow))) "Undefined" "MultiplyWithRoot" 0 0)))

(event EventBeginPlay
  (Utilities|Time|SetTimerbyEvent (delegate Custom|Fire) 0.1 true))

(fn ConstructionScript)